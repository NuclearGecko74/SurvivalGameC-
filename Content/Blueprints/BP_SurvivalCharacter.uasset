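; BP_SurvivalCharacter is a character Blueprint with a socket-mounted camera and modular body and gear meshes.
; The construction script attaches the camera to the main mesh's CameraSocket, keeping relative transforms.
; It sets that mesh as master pose for the chest, helmet, feet, vest, hands, backpack and leg meshes, so they share its animation.
; The event graph holds only empty event stubs.
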(event `self.ReceiveBeginPlay`)

(fn `UserConstructionScript`
  (`SceneComponent.K2_AttachToComponent` (`self.CameraComp`) (`self.Mesh`) "CameraSocket" "KeepRelative" "KeepRelative" "KeepRelative" true)
  (`SkinnedMeshComponent.SetLeaderPoseComponent` (`self.ChestMesh`) (`self.Mesh`) false)
  (`SkinnedMeshComponent.SetLeaderPoseComponent` (`self.HelmetMesh`) (`self.Mesh`) false)
  (`SkinnedMeshComponent.SetLeaderPoseComponent` (`self.FeetMesh`) (`self.Mesh`) false)
  (`SkinnedMeshComponent.SetLeaderPoseComponent` (`self.VestMesh`) (`self.Mesh`) false)
  (`SkinnedMeshComponent.SetLeaderPoseComponent` (`self.HandsMesh`) (`self.Mesh`) false)
  (`SkinnedMeshComponent.SetLeaderPoseComponent` (`self.BackpackMesh`) (`self.Mesh`) false)
  (`SkinnedMeshComponent.SetLeaderPoseComponent` (`self.LegsMesh`) (`self.Mesh`) false))